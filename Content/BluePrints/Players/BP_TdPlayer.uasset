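; Player camera actor (BP_TdPlayer) that provides edge-scroll panning and mouse-wheel zoom.
; Each Tick, helper functions compare the cursor position with the viewport edges within a small tolerance to produce direction flags.
; Those flags feed two move functions that offset the actor along world X and Y by CameraMoveSpeed, without sweep.
; The wheel steps SpringArm TargetArmLength by CameraSpeed, checked against upper and lower limits.
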(event EventBeginPlay)

(event Collision|EventActorBeginOverlap
  (params (OtherActor :type Actor%20Object%20Reference)))

(event EventTick
  (params (DeltaSeconds :type Float%20%28single-precision%29))
  (bind (_isright _isleft) (|判断相机是否该左右移动))
  (bind (_isup _isdown) (|判断是否该上下移动))
  (Utilities|FlowControl|Sequence
    (:then_0
      (|相机上下移动 _isup _isdown))
    (:then_1
      (|相机左右移动 _isright _isleft))))

(event Input|MouseEvents|MouseWheelUp
  (params (Key :type Key%20Structure :default "AnyKey"))
  (bind _springarm (Variables|Default|GetSpringArm))
  ;[1 1 1] Camera +/-
  (:Pressed
    (if (> (Variables|/Script/Engine.SpringArmComponent|GetTargetArmLength _springarm) -5e+02)
      (Variables|/Script/Engine.SpringArmComponent|SetTargetArmLength _springarm (- (Variables|/Script/Engine.SpringArmComponent|GetTargetArmLength _springarm) (Variables|Default|GetCameraSpeed))))))

(event Input|MouseEvents|MouseWheelDown
  (params (Key :type Key%20Structure :default "AnyKey"))
  (bind _springarm (Variables|Default|GetSpringArm))
  ;[1 1 1] Camera +/-
  (:Pressed
    (if (< (Variables|/Script/Engine.SpringArmComponent|GetTargetArmLength _springarm) 1e+03)
      (Variables|/Script/Engine.SpringArmComponent|SetTargetArmLength _springarm (+ (Variables|/Script/Engine.SpringArmComponent|GetTargetArmLength _springarm) (Variables|Default|GetCameraSpeed))))))

(fn ConstructionScript)