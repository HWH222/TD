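; AI controller that drives a possessed BP_Tower to aim at and attack enemies.
; It stores the pawn on possession, and a looping half-second timer started at BeginPlay calls AimOnEnemy.
; That event casts the pawn to BP_Tower and passes the first EnemyArray entry to RotateToEnemy and Attack, with no check for an empty array.
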(event Custom|AimOnEnemy
  (bind _asbp_tower (Utilities|Casting|CastToBP_Tower (Variables|Default|GetTower)))
  (Default|RotatetoEnemy _asbp_tower (Utilities|Array|Get(acopy) (Variables|/Game/BluePrints/Tower/BP_Tower.BP_Tower_C|GetEnemyArray _asbp_tower)))
  (Default|Attack _asbp_tower (Utilities|Array|Get(acopy) (Variables|/Game/BluePrints/Tower/BP_Tower.BP_Tower_C|GetEnemyArray _asbp_tower))))

(event EventBeginPlay
  (Utilities|Time|SetTimerbyFunctionName self "AimOnEnemy" 0.5 true))

(event EventOnPossess
  (params (PossessedPawn :type Pawn%20Object%20Reference))
  (Variables|Default|SetTower PossessedPawn))

(fn ConstructionScript)