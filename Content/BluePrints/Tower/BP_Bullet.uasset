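; BP_Bullet is a tower projectile that homes in on a given enemy and damages it on contact.
; AttacktoEnemy faces the enemy once, then loops on a short Delay, moving the bullet a fixed step toward the enemy's current location without sweeping.
; The sphere overlap applies SumOfDamage to any BP_Enemy it touches and destroys the bullet.
; A lifespan set at BeginPlay removes bullets that never hit.
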(event OnComponentBeginOverlap(Sphere)
  (params (OverlappedComponent :type Primitive%20Component%20Object%20Reference) (OtherActor :type Actor%20Object%20Reference) (OtherComp :type Primitive%20Component%20Object%20Reference) (OtherBodyIndex :type Integer) (bFromSweep :type Boolean) (SweepResult :type Hit%20Result%20Structure%20%28by%20ref%29))
  (bind _asbp_enemy (Utilities|Casting|CastToBP_Enemy OtherActor))
  (Game|Damage|ApplyDamage _asbp_enemy (Variables|Default|GetSum%20of%20Damage) 0 0)
  (Actor|DestroyActor))

(event Custom|Attack%20to%20Enemy
  (params (Enemy :type Actor%20Object%20Reference))
  (bind _returnvalue (Transformation|GetActorLocation))
  (bind _returnvalue_2 (Transformation|GetActorLocation Enemy))
  (bind _returnvalue_3 (Math|Rotator|FindLookatRotation _returnvalue _returnvalue_2))
  (Transformation|SetActorRotation _returnvalue_3)
  (Transformation|AddActorWorldOffset (* (Math|Vector|GetForwardVector _returnvalue_3) 5e+01) :!label _label)
  (Utilities|FlowControl|Delay 0.01)
  (goto _label))

(event EventBeginPlay
  (Actor|SetLifeSpan 5.0))

(fn ConstructionScript)